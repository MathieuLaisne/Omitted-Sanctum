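; BP_WordControlRoom is a box volume that punishes players for saying a banned word while inside it.
; On overlap it binds WordEvaluation to the player's Speaking event, and unbinds it when the player leaves.
; If the spoken words contain BannedWord, it gives the configured Curse to player index 0's OSPlayerState.
; The construction script sizes the box from Bounds, and a debug flag draws it and logs curses.
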(event `self.ReceiveBeginPlay`
  (if (`self.IsDebug`)
    (`KismetSystemLibrary.DrawDebugBox` (`SceneComponent.K2_GetComponentLocation` (`self.Box`)) (`self.Bounds`) (struct :`G` 0.145292 :`B` 1.0 :`A` 1.0) (struct) 10000.0 1.0)))

(event `self.ReceiveActorBeginOverlap`
  (params (OtherActor :type "Actor Object Reference"))
  (bind _asbp_player (cast `/Game/Player/BP_Player` OtherActor))
  (bind _output_get (set `self.Player` _asbp_player))
  (add `/Game/Player/BP_Player.Speaking` _output_get (delegate `WordEvaluation`)))

(event `WordEvaluation`
  (params (Words :type "Array of /Game/Words Enum (by ref)"))
  (if (`KismetArrayLibrary.Array_Contains` Words (`self.BannedWord`))
    (if (`self.IsDebug`)
      (`KismetSystemLibrary.PrintText` "Applying curses"))
    (bind _asosplayer_state (cast `/Game/Blueprints/OSPlayerState` (`GameplayStatics.GetPlayerState` 0)))
    (`/Game/Blueprints/OSPlayerState.GiveCurse` _asosplayer_state (`self.Curse`))))

(event `self.ReceiveActorEndOverlap`
  (params (OtherActor :type "Actor Object Reference"))
  (bind _asbp_player (cast `/Game/Player/BP_Player` OtherActor))
  (remove `/Game/Player/BP_Player.Speaking` _asbp_player (delegate `WordEvaluation`)))

(fn `UserConstructionScript`
  (`BoxComponent.SetBoxExtent` (`self.Box`) (`self.Bounds`) true))