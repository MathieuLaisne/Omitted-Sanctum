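; BP_WordControlRoom is a room volume that punishes the player for speaking a banned word inside it.
; The construction script sizes its box from a bounds variable, and overlap begin and end bind and unbind the player's speaking event.
; Spoken words are checked for the banned word; a match gives the configured curse to player state index 0.
; A debug flag draws the box and prints when curses apply.
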(event `self.ReceiveBeginPlay`
  (if (`self.IsDebug`)
    (`KismetSystemLibrary.DrawDebugBox` (`SceneComponent.K2_GetComponentLocation` (`self.Box_0`)) (`self.Bounds_0`) (struct :`G` 0.145292 :`B` 1.0 :`A` 1.0) (struct) 10000.0 1.0)))

(event `self.ReceiveActorBeginOverlap`
  (params (OtherActor :type "Actor Object Reference"))
  (bind _asbp_player (cast `/Game/Player/BP_Player` OtherActor))
  (bind _output_get (set `self.Player` _asbp_player))
  (add `/Game/Player/BP_Player.Speaking` _output_get (delegate `SpellEvaluation`)))

(event `SpellEvaluation`
  (params (Words :type "OSMagicSpell Structure"))
  (bind _returnvalue (`MagicHelperLibrary.SpellContainWord` Words (`self.BannedWord`)))
  (if _returnvalue
    (if (`self.IsDebug`)
      (`KismetSystemLibrary.PrintText` "Applying curses"))
    (bind _asosplayer_state (cast `/Game/Blueprints/OSPlayerState` (`GameplayStatics.GetPlayerState` 0)))
    (`/Game/Blueprints/OSPlayerState.GiveCurse` _asosplayer_state (`self.Curse_0`))))

(event `self.ReceiveActorEndOverlap`
  (params (OtherActor :type "Actor Object Reference"))
  (bind _asbp_player (cast `/Game/Player/BP_Player` OtherActor))
  (remove `/Game/Player/BP_Player.Speaking` _asbp_player (delegate `SpellEvaluation`)))

(fn `UserConstructionScript`
  (`BoxComponent.SetBoxExtent` (`self.Box_0`) (`self.Bounds_0`) true))