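; BP_Spellbook is a world item that displays a floating name and description label for a spellbook; it holds no pickup or spell logic.
; On BeginPlay it passes its ItemName and ItemDesc to its UW_ItemBoxText widget.
; InteractionTrigger overlaps show and hide the widget without filtering the overlapping actor.
; While visible, the widget billboards each Tick toward a point slightly above the player camera.
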(event `self.ReceiveBeginPlay`
  (bind _asuw_item_box_text (cast `/Game/UI/UW_ItemBoxText` (`WidgetComponent.GetWidget` (`self.Widget`))))
  (`/Game/UI/UW_ItemBoxText.SetNameAndDesc` _asuw_item_box_text (`self.ItemName`) (`self.ItemDesc`)))

(event `self.ReceiveTick`
  (params (DeltaSeconds :type "Float (single-precision)"))
  (bind _widget (`self.Widget`))
  (if (`self.IsVisible`)
    (`SceneComponent.K2_SetWorldRotation` _widget (`KismetMathLibrary.FindLookAtRotation` (`SceneComponent.K2_GetComponentLocation` _widget) (+ (`self.K2_GetActorLocation` (`GameplayStatics.GetPlayerCameraManager` 0)) (0.0 0.0 70.0))) false false)))

(event `self.InteractionTrigger.OnComponentBeginOverlap`
  (params (OverlappedComponent :type "PrimitiveComponent Object Reference") (OtherActor :type "Actor Object Reference") (OtherComp :type "PrimitiveComponent Object Reference") (OtherBodyIndex :type Integer) (bFromSweep :type Boolean) (SweepResult :type "HitResult Structure (by ref)"))
  (`SceneComponent.SetVisibility` (`self.Widget`) true false)
  (set `self.IsVisible` true))

(event `self.InteractionTrigger.OnComponentEndOverlap`
  (params (OverlappedComponent :type "PrimitiveComponent Object Reference") (OtherActor :type "Actor Object Reference") (OtherComp :type "PrimitiveComponent Object Reference") (OtherBodyIndex :type Integer))
  (`SceneComponent.SetVisibility` (`self.Widget`) false false)
  (set `self.IsVisible` false))

(fn `UserConstructionScript`)