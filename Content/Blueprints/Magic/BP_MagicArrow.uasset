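; BP_MagicArrow is a magic projectile that damages BP_Enemies actors and can pierce through them.
; Tick moves it along its forward vector by Speed per frame, without delta time or sweep.
; Enemy overlaps spend a penetration charge to apply elemental damage and effects; at zero charges it destroys itself without damage, as do non-enemy overlaps.
; The construction script configures its Niagara component's shape, size and particle amount.
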(event `self.ReceiveActorBeginOverlap`
  (params (OtherActor :type "Actor Object Reference"))
  (bind (_element_name _element_canapplytoself _element_canapplytocaster _element_canapplyonhit) (break `OSMagicElement` (`self.Element`)))
  (bind _asbp_enemies (cast `/Game/Enemies/BP_Enemies` OtherActor)
    (:`then`
      (if (== (`self.PenetrativeAmount`) 0)
        (`self.K2_DestroyActor`)
        (else
          (`/Engine/EditorBlueprintResources/StandardMacros.DecrementInt` (`self.PenetrativeAmount`)
            (:`  `
              (`/Game/Enemies/BP_Enemies.ApplyMagicDamage` _asbp_enemies _element_name (`self.Damage`) _element_canapplyonhit (`self.EffectDuration`)))))))
    (:`CastFailed`
      (`self.K2_DestroyActor`))))

(event `self.ReceiveTick`
  (params (DeltaSeconds :type "Float (single-precision)"))
  (`self.K2_SetActorLocation` (+ (`self.K2_GetActorLocation`) (* (`self.GetActorForwardVector`) (`self.Speed`) 1.0))))

(fn `UserConstructionScript`
  (bind _niagaracomponent (`self.NiagaraComponent`))
  (`NiagaraComponent.SetVariableFloat` _niagaracomponent "Radius" 5.0)
  (`NiagaraComponent.SetVariableFloat` _niagaracomponent "FluidRadius" 0.95)
  (`NiagaraComponent.SetVariableVec3` _niagaracomponent "NonUniformScale" (3.0 0.1 0.0))
  (`NiagaraComponent.SetVariableVec3` _niagaracomponent "WorldSize" (200.0 50.0 15.0))
  (`NiagaraComponent.SetVariableFloat` _niagaracomponent "ParticleAmount" 3000.0))