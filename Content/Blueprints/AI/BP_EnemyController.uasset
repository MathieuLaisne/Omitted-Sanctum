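; AI controller for enemies that runs the BasicEnemies behavior tree and starts the PathIndex blackboard key at zero.
; Each perception update goes to sight and hearing handlers, which filter by sense class and write to the blackboard.
; Sight sets TargetActor to the player character, whichever actor was sensed, or clears it on loss and saves LastKnownLocation.
; Hearing stores the stimulus position as TargetLocation and prints a debug message.
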(event `self.ReceiveBeginPlay`
  (`self.RunBehaviorTree` "/Game/Blueprints/AI/BasicEnemies.BasicEnemies")
  (`BlackboardComponent.SetValueAsInt` (`AIBlueprintHelperLibrary.GetBlackboard` null) "PathIndex" 0))

(event `self.AIPerception.OnTargetPerceptionUpdated`
  (params (Actor :type "Actor Object Reference") (Stimulus :type "AIStimulus Structure"))
  (`self.Handle Sight Perception` Actor Stimulus)
  (`self.Handle Hearing Perception` Actor Stimulus))

(fn `Handle Hearing Perception`
  (params (Actor :type "Actor Object Reference") (Sitmulus :type "AIStimulus Structure"))
  (bind _returnvalue (`AIPerceptionSystem.GetSenseClassForStimulus` Sitmulus))
  (if (== _returnvalue "/Script/AIModule.AISense_Hearing")
    (`BlackboardComponent.SetValueAsVector` (`AIBlueprintHelperLibrary.GetBlackboard` null) "TargetLocation" (`.StimulusLocation` (break `AIStimulus` Sitmulus)))
    (`KismetSystemLibrary.PrintString` "I hear noise")))

(fn `Handle Sight Perception`
  (params (Actor :type "Actor Object Reference") (Stimulus :type "AIStimulus Structure"))
  (bind (_age _expirationage _strength _stimuluslocation _receiverlocation _tag _bsuccessfullysensed) (break `AIStimulus` Stimulus))
  (bind _returnvalue (`AIPerceptionSystem.GetSenseClassForStimulus` Stimulus))
  (if (== _returnvalue "/Script/AIModule.AISense_Sight")
    (`BlackboardComponent.SetValueAsObject` (`AIBlueprintHelperLibrary.GetBlackboard` null) "TargetActor" (`KismetMathLibrary.SelectObject` (`GameplayStatics.GetPlayerCharacter` 0) null _bsuccessfullysensed))
    (if (not _bsuccessfullysensed)
      (`BlackboardComponent.SetValueAsVector` (`AIBlueprintHelperLibrary.GetBlackboard` null) "LastKnownLocation" _stimuluslocation))))

(fn `UserConstructionScript`)