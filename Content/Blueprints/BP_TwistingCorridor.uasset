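; Corridor actor that twists its dynamic mesh once when the player first enters, notifying OSPlayerState at start and finish.
; A timeline applies the same twist warp to the corridor and a hidden, thin ghost strip offset below it.
; Afterwards the strip's vertices become spline points, then it is released.
; Tick eases the overlapping player's gravity toward the nearest spline point, and leaving restores the gravity saved when twisting began.
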(event `self.ReceiveActorBeginOverlap`
  (params (OtherActor :type "Actor Object Reference"))
  (if (== OtherActor (`GameplayStatics.GetPlayerPawn` 0))
    (bind _asbp_player (cast `/Game/Player/BP_Player` (`GameplayStatics.GetPlayerPawn` 0)))
    (set `self.Player` _asbp_player)
    (if (not (`self.IsDeforming`))
      ;[1 1 1] MC Message For Reaction
      (bind _asosplayer_state (cast `/Game/Blueprints/OSPlayerState` (`GameplayStatics.GetPlayerState` 0)))
      (`/Game/Blueprints/OSPlayerState.OnDeformedStarted` _asosplayer_state)
      (set `self.IsDeforming` true)
      (set `self.InitialGravity` (`CharacterMovementComponent.GetGravityDirection` (`Character.CharacterMovement` (`self.Player`))))
      (bind (_direction _alpha) (`Timeline|Timeline` :!via `PlayFromStart`)
        (:`Update`
          (bind _returnvalue (* _alpha (`self.TwistAngle`)))
          (`GeometryScriptLibrary_MeshDeformFunctions.ApplyTwistWarpToMesh` (`self.Dynamic Mesh`) (make `GeometryScriptTwistWarpOptions` true 0.0) (`KismetMathLibrary.MakeTransform` (`self.Twist Start`) (`self.Twist Rotation`)) _returnvalue (`self.Corridor Length`) null)
          (`GeometryScriptLibrary_MeshDeformFunctions.ApplyTwistWarpToMesh` (`self.GhostMesh`) (make `GeometryScriptTwistWarpOptions` true 0.0) (`KismetMathLibrary.MakeTransform` (`self.Twist Start`) (`self.Twist Rotation`)) _returnvalue (`self.Corridor Length`) null))
        (:`Finished`
          (`/Game/Blueprints/OSPlayerState.OnDeformedFinished` _asosplayer_state)
          (set `self.IsDeformed` true)
          (`self.Update Spline`)
          (`self.ReleaseComputeMesh` (`self.GhostMesh`)))))))

(event `self.ReceiveActorEndOverlap`
  (params (OtherActor :type "Actor Object Reference"))
  (bind _player (`self.Player`))
  (if (== OtherActor _player)
    (`CharacterMovementComponent.SetGravityDirection` (`Character.CharacterMovement` _player) (`self.InitialGravity`))
    (set `self.Player` null)))

(event `self.ReceiveTick`
  (params (DeltaSeconds :type "Float (single-precision)"))
  (bind _player (`self.Player`))
  (bind _charactermovement (`Character.CharacterMovement` _player))
  (bind _returnvalue (`SceneComponent.K2_GetComponentLocation` (`Character.CapsuleComponent` _player)))
  (if (`self.IsDeformed`)
    (`/Engine/EditorBlueprintResources/StandardMacros.IsValid` (`self.Player`)
      (:`Is Valid`
        (`CharacterMovementComponent.SetGravityDirection` _charactermovement (`KismetMathLibrary.VInterpTo` (`CharacterMovementComponent.GetGravityDirection` _charactermovement) (`KismetMathLibrary.GetDirectionUnitVector` _returnvalue (`SplineComponent.FindLocationClosestToWorldLocation` (`self.Spline`) _returnvalue "World")) DeltaSeconds 5.0))))))

(fn `BaseSpline`
  (bind _spline (`self.Spline`))
  (for _index (range (+ (`SplineComponent.GetNumberOfSplinePoints` _spline) 1))
    (bind (_returnvalue_x _returnvalue_y) (`KismetMathLibrary.BreakVector` (`SplineComponent.GetLocationAtSplinePoint` _spline _index "Local")))
    (`SplineComponent.SetLocationAtSplinePoint` _spline _index (`KismetMathLibrary.MakeVector` 0.0 _returnvalue_y -100.0) "Local" true)))

(fn `RebuildMesh`
  (bind _returnvalue (`BaseDynamicMeshComponent.GetDynamicMesh` (`self.DynamicMeshComponent`)))
  (bind _output_get (set `self.Dynamic Mesh` _returnvalue))
  (bind _returnvalue_2 (`GeometryScriptLibrary_MeshNormalsFunctions.RecomputeNormals` _output_get (struct) false null))
  (bind _returnvalue_3 (`GeometryScriptLibrary_CollisionFunctions.SetDynamicMeshCollisionFromMesh` _returnvalue_2 (`self.DynamicMeshComponent`) (struct) null))
  (`GeometryScriptLibrary_StaticMeshFunctions.CopyMeshFromStaticMesh` (`self.MeshToDeform`) _returnvalue_3 (make `GeometryScriptCopyMeshFromAssetOptions` true) (struct) null))

(fn `Update Spline`
  (bind _spline (`self.Spline`))
  (bind _positionlist (`GeometryScriptLibrary_MeshQueryFunctions.GetAllVertexPositions` (`self.GhostMesh`) true))
  (bind _vectorarray (`GeometryScriptLibrary_ListUtilityFunctions.ConvertVectorListToArray` _positionlist))
  (`SplineComponent.ClearSplinePoints` _spline true)
  (bind (_output_x _output_y _output_z) (`KismetMathLibrary.BreakVector` (`|GetArrayItem` _vectorarray)))
  (`SplineComponent.AddSplinePoint` _spline (`KismetMathLibrary.MakeVector` 0.0 (- _output_y 100.0) _output_z) "Local" true)
  (for _array_element _vectorarray
    (`SplineComponent.AddSplinePoint` _spline _array_element "Local" true))
  (`SplineComponent.AddSplinePoint` _spline (`KismetMathLibrary.MakeVector` 0.0 (+ (.y _array_element) 100.0) (.z _array_element)) "Local" true))

(fn `UserConstructionScript`
  (bind _corridor_length (`self.Corridor Length`))
  (bind _returnvalue (`BaseDynamicMeshComponent.GetDynamicMesh` (`self.DynamicMeshComponent`)))
  (bind _output_get (set `self.Dynamic Mesh` _returnvalue))
  (bind _returnvalue_2 (`GeometryScriptLibrary_MeshNormalsFunctions.RecomputeNormals` _output_get (struct) false null))
  (`GeometryScriptLibrary_CollisionFunctions.SetDynamicMeshCollisionFromMesh` _returnvalue_2 (`self.DynamicMeshComponent`) (struct) null)
  (bind _returnvalue_3 (`self.AllocateComputeMesh`))
  (bind _output_get_2 (set `self.GhostMesh` _returnvalue_3))
  (`GeometryScriptLibrary_MeshPrimitiveFunctions.AppendRectangleXY` _output_get_2 (struct) (`KismetMathLibrary.MakeTransform` (0.0 0.0 -250.0)) 0.1 _corridor_length 0 (/ (`KismetMathLibrary.FTrunc` _corridor_length) 20) null))