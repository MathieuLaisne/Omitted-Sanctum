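; Map generator that builds a floor's room layout on BeginPlay, based on Difficulty and Floor.
; Difficulty selects rooms from the RoomList data table by type combination and scales MaxRooms above the lowest level.
; Floor then sets key-room or boss flags for GenerateRoomLayout, with MaxRooms as grid size.
; SpawnRooms currently does nothing, as its grid-to-BP_Room spawning loop is disconnected.
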(event `self.ReceiveBeginPlay`
  (`self.Generate Floor`)
  (`self.Spawn Rooms`))

(fn `AddAllRoomsInDT`
  (params (Data :type "Array of OSRoomData Structure"))
  (bind _roomlist (`self.RoomList`))
  (bind _outrownames (`DataTableFunctionLibrary.GetDataTableRowNames` _roomlist))
  (for _array_element _outrownames
    (bind _returnvalue (`|GetDataTableRow` _roomlist _array_element)
      (:`then`
        (`KismetArrayLibrary.Array_Add` Data _returnvalue))))
  (return))

(fn `AddAllSoloRoomsInDT`
  (params (Data :type "Array of OSRoomData Structure"))
  (bind _roomlist (`self.RoomList`))
  (bind _outrownames (`DataTableFunctionLibrary.GetDataTableRowNames` _roomlist))
  (for _array_element _outrownames
    (bind _returnvalue (`|GetDataTableRow` _roomlist _array_element)
      (:`then`
        (if (`self.IsSoloRoom` (`.Types` (break `OSRoomData` _returnvalue)))
          (`KismetArrayLibrary.Array_Add` Data _returnvalue)))))
  (return))

(fn `AddNoPuzzleRoomsInDT`
  (params (Data :type "Array of OSRoomData Structure"))
  (bind _roomlist (`self.RoomList`))
  (bind _outrownames (`DataTableFunctionLibrary.GetDataTableRowNames` _roomlist))
  (for _array_element _outrownames
    (bind _returnvalue (`|GetDataTableRow` _roomlist _array_element)
      (:`then`
        (if (not (`self.IsPuzzleRoom` (`.Types` (break `OSRoomData` _returnvalue))))
          (`KismetArrayLibrary.Array_Add` Data _returnvalue)))))
  (return))

(fn `AddNoSoloRoomsInDT`
  (params (Data :type "Array of OSRoomData Structure"))
  (bind _roomlist (`self.RoomList`))
  (bind _outrownames (`DataTableFunctionLibrary.GetDataTableRowNames` _roomlist))
  (for _array_element _outrownames
    (bind _returnvalue (`|GetDataTableRow` _roomlist _array_element)
      (:`then`
        (if (not (`self.IsSoloRoom` (`.Types` (break `OSRoomData` _returnvalue))))
          (`KismetArrayLibrary.Array_Add` Data _returnvalue)))))
  (return))

(fn `AddPlatformerEnemyRoomsInDT`
  (params (Data :type "Array of OSRoomData Structure"))
  (bind _roomlist (`self.RoomList`))
  (bind _outrownames (`DataTableFunctionLibrary.GetDataTableRowNames` _roomlist))
  (for _array_element _outrownames
    (bind _returnvalue (`|GetDataTableRow` _roomlist _array_element)
      (:`then`
        (if (`self.IsPlatformerEnemyRoom` (`.Types` (break `OSRoomData` _returnvalue)))
          (`KismetArrayLibrary.Array_Add` Data _returnvalue)))))
  (return))

(fn `AddPuzzleEnemyRoomsInDT`
  (params (Data :type "Array of OSRoomData Structure"))
  (bind _roomlist (`self.RoomList`))
  (bind _outrownames (`DataTableFunctionLibrary.GetDataTableRowNames` _roomlist))
  (for _array_element _outrownames
    (bind _returnvalue (`|GetDataTableRow` _roomlist _array_element)
      (:`then`
        (if (`self.IsPuzzleEnemyRoom` (`.Types` (break `OSRoomData` _returnvalue)))
          (`KismetArrayLibrary.Array_Add` Data _returnvalue)))))
  (return))

(fn `Generate Floor`
  (locals (AvailableRooms :type "Array of OSRoomData Structure"))
  (switch `int` (`self.Difficulty`)
    (:`0`
      (`self.AddAllSoloRoomsInDT` (`local.AvailableRooms`)))
    (:`1`
      (`self.AddAllSoloRoomsInDT` (`local.AvailableRooms`))
      (`self.AddPuzzleEnemyRoomsInDT` (`local.AvailableRooms`))
      (set `self.MaxRooms` (* (`self.MaxRooms`) 1.5)))
    (:`2`
      (`self.AddAllSoloRoomsInDT` (`local.AvailableRooms`))
      (`self.AddPuzzleEnemyRoomsInDT` (`local.AvailableRooms`))
      (`self.AddPlatformerEnemyRoomsInDT` (`local.AvailableRooms`))
      (set `self.MaxRooms` (* (`self.MaxRooms`) 2)))
    (:`3`
      (`self.AddNoPuzzleRoomsInDT` (`local.AvailableRooms`))
      (set `self.MaxRooms` (* (`self.MaxRooms`) 2.5)))
    (:`4`
      (`self.AddNoSoloRoomsInDT` (`local.AvailableRooms`))
      (set `self.MaxRooms` (* (`self.MaxRooms`) 3))))
  (switch `int` (`self.Floor`)
    (:`0`
      (`self.GenerateRoomLayout` (`local.AvailableRooms`) (`self.MaxRooms`)))
    (:`1`
      (`self.GenerateRoomLayout` (`local.AvailableRooms`) (`self.MaxRooms`) true))
    (:`2`
      (`self.GenerateRoomLayout` (`local.AvailableRooms`) (`self.MaxRooms`) false true :!label _label))
    (:`3`
      (goto _label))))

(fn `Spawn Rooms`
  (locals (X :type "Float (double-precision)" :default 0.0) (Y :type "Float (double-precision)" :default 0.0)))

(fn `UserConstructionScript`)