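; OSPlayerState tracks the player's health, bandages, curses and kill target.
; Damage lowers HP with no death handling yet, while healing spends a bandage and restores HP when a timeline finishes.
; GiveCurse merges stacks with a cap, raises EnemiesToKill and derives SpeedPercentage from one curse type; RemoveCurse drops the strongest curse.
; Deformation events print reaction text copied from BP_Player, indexed by a counter of deformations seen.
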(event `self.ReceiveBeginPlay`
  (set `self.CurrentHP` (`self.MaxHP`))
  (bind _asbp_player (cast `/Game/Player/BP_Player` (`GameplayStatics.GetPlayerPawn` 0)))
  (set `self.ReactionToDeformation` (`/Game/Player/BP_Player.ReactionToDeformation` _asbp_player))
  (set `self.ReactionToDeformationEnd` (`/Game/Player/BP_Player.ReactionToDeformationEnd` _asbp_player)))

(event `TakeDamage`
  (params (Damage :type Integer))
  (bind _output_get (set `self.CurrentHP` (- (`self.CurrentHP`) Damage)))
  (if (<= _output_get 0)
    _))

(event `Heal`
  (bind _bandageamount (`self.BandageAmount`))
  (if (not (<= _bandageamount 0))
    (set `self.BandageAmount` (- _bandageamount 1))
    (`Timeline|Healing` :!via `PlayFromStart`
      (:`Finished`
        (set `self.CurrentHP` (`KismetMathLibrary.Clamp` (+ (`self.CurrentHP`) 15) 0 (`self.MaxHP`)))))))

(event `OnDeformedStarted`
  (`KismetSystemLibrary.PrintText` (`BlueprintMapLibrary.Map_Find` (`self.ReactionToDeformation`) (`self.DeformationSeen`))))

(event `OnDeformedFinished`
  (`KismetSystemLibrary.PrintText` (`BlueprintMapLibrary.Map_Find` (`self.ReactionToDeformationEnd`) (`self.DeformationSeen`)))
  (`/Engine/EditorBlueprintResources/StandardMacros.IncrementInt` (`self.DeformationSeen`)))

(fn `GiveCurse`
  (params (Curse :type "Map of /Game/Weapon/CurseType Enum to Integer"))
  (bind _curses (`self.Curses`))
  (bind (_value _returnvalue) (`BlueprintMapLibrary.Map_Find` (`self.Curses`) "NewEnumerator0"))
  (bind _keys (`BlueprintMapLibrary.Map_Keys` Curse))
  (for _array_element _keys
    (if (`BlueprintMapLibrary.Map_Contains` _curses _array_element)
      (bind _value_2 (`BlueprintMapLibrary.Map_Find` Curse _array_element))
      (`BlueprintMapLibrary.Map_Add` _curses _array_element (`KismetMathLibrary.Clamp` (+ _value_2 (`BlueprintMapLibrary.Map_Find` _curses _array_element)) 0 75))
      (else
        (`BlueprintMapLibrary.Map_Add` _curses _array_element _value_2))))
  (set `self.EnemiesToKill` (+ (`self.EnemiesToKill`) (`self.DifficultyInfo`)))
  (if _returnvalue
    (set `self.SpeedPercentage` (- 1.0 (* _value 0.01)))
    (else
      (set `self.SpeedPercentage` 1.0))))

(fn `RemoveCurse`
  (locals (MaxFound :type Integer) (MaxIndex :type Integer))
  (bind _curses (`self.Curses`))
  (bind _curses_2 (`self.Curses`))
  (bind _values (`BlueprintMapLibrary.Map_Values` _curses))
  (for (_array_element _array_index) _values
    (if (> _array_element (`local.MaxFound`))
      (set `local.MaxFound` _array_element)
      (set `local.MaxIndex` _array_index)))
  (bind _keys (`BlueprintMapLibrary.Map_Keys` _curses))
  (`BlueprintMapLibrary.Map_Remove` _curses_2 (`|GetArrayItem` _keys (`local.MaxIndex`)))
  (if (not (`BlueprintMapLibrary.Map_IsEmpty` _curses_2))
    (set `self.EnemiesToKill` (`self.DifficultyInfo`))))

(fn `UserConstructionScript`)