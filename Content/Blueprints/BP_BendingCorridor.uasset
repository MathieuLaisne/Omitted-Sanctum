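; Corridor actor that bends once when the player first enters, then redirects their gravity to suit the curved shape.
; A timeline drives a Geometry Script bend warp on the dynamic mesh and notifies the player state at start and finish.
; Once bent, Tick points gravity toward the closest spline point in the XZ plane, and leaving restores the saved direction.
; Helper functions lay out spline points and rebuild mesh and collision.
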(event `self.ReceiveActorBeginOverlap`
  (params (OtherActor :type "Actor Object Reference"))
  (if (== OtherActor (`GameplayStatics.GetPlayerPawn` 0))
    (bind _asbp_player (cast `/Game/Player/BP_Player` (`GameplayStatics.GetPlayerPawn` 0)))
    (set `self.Player` _asbp_player)
    (if (not (`self.IsDeforming`))
      ;[1 1 1] MC Message For Reaction
      (bind _asosplayer_state (cast `/Game/Blueprints/OSPlayerState` (`GameplayStatics.GetPlayerState` 0)))
      (`/Game/Blueprints/OSPlayerState.OnDeformedStarted` _asosplayer_state)
      (set `self.IsDeforming` true)
      (set `self.InitialGravity` (`CharacterMovementComponent.GetGravityDirection` (`Character.CharacterMovement` (`self.Player`))))
      (bind (_direction _alpha) (`Timeline|Timeline` :!via `PlayFromStart`)
        (:`Update`
          (`GeometryScriptLibrary_MeshDeformFunctions.ApplyBendWarpToMesh` (`self.Dynamic Mesh`) (make `GeometryScriptBendWarpOptions` true) (`KismetMathLibrary.MakeTransform` (`self.Twist Start`) (`self.Bend Rotation`)) (* _alpha (`self.BendAngle`)) (`self.Corridor Length`) null))
        (:`Finished`
          (`/Game/Blueprints/OSPlayerState.OnDeformedFinished` _asosplayer_state)
          (set `self.IsDeformed` true))))))

(event `self.ReceiveActorEndOverlap`
  (params (OtherActor :type "Actor Object Reference"))
  (bind _player (`self.Player`))
  (if (== OtherActor _player)
    (`CharacterMovementComponent.SetGravityDirection` (`Character.CharacterMovement` _player) (`self.InitialGravity`))
    (set `self.Player` null)))

(event `self.ReceiveTick`
  (params (DeltaSeconds :type "Float (single-precision)"))
  (bind _player (`self.Player`))
  (bind _returnvalue (`SceneComponent.K2_GetComponentLocation` (`Character.CapsuleComponent` _player)))
  (bind (_returnvalue_x _returnvalue_y _returnvalue_z) (`KismetMathLibrary.BreakVector` (`KismetMathLibrary.GetDirectionUnitVector` _returnvalue (`SplineComponent.FindLocationClosestToWorldLocation` (`self.Spline`) _returnvalue "World"))))
  (if (`self.IsDeformed`)
    (`/Engine/EditorBlueprintResources/StandardMacros.IsValid` (`self.Player`)
      (:`Is Valid`
        (`CharacterMovementComponent.SetGravityDirection` (`Character.CharacterMovement` _player) (`KismetMathLibrary.MakeVector` _returnvalue_x 0.0 _returnvalue_z))))))

(fn `BaseSpline`
  (bind _spline (`self.Spline`))
  (for _index (range (+ (`SplineComponent.GetNumberOfSplinePoints` _spline) 1))
    (`SplineComponent.SetLocationAtSplinePoint` _spline _index (`KismetMathLibrary.MakeVector` 0.0 (- (* _index 50.0) 500.0) -100.0) "Local" true)))

(fn `RebuildMesh`
  (bind _returnvalue (`BaseDynamicMeshComponent.GetDynamicMesh` (`self.DynamicMeshComponent`)))
  (bind _output_get (set `self.Dynamic Mesh` _returnvalue))
  (bind _returnvalue_2 (`GeometryScriptLibrary_MeshNormalsFunctions.RecomputeNormals` _output_get (struct) false null))
  (bind _returnvalue_3 (`GeometryScriptLibrary_CollisionFunctions.SetDynamicMeshCollisionFromMesh` _returnvalue_2 (`self.DynamicMeshComponent`) (struct) null))
  (`GeometryScriptLibrary_StaticMeshFunctions.CopyMeshFromStaticMesh` (`self.MeshToDeform`) _returnvalue_3 (make `GeometryScriptCopyMeshFromAssetOptions` true) (struct) null))

(fn `ToBend`
  (bind _spline (`self.Spline`))
  (bind _returnvalue (- (`SplineComponent.GetNumberOfSplinePoints` _spline) 1))
  (for _index (range 2 (+ _returnvalue 1))
    (bind _returnvalue_x (`KismetMathLibrary.BreakVector` (`SplineComponent.GetLocationAtSplinePoint` _spline _index "Local")))
    (bind _returnvalue_2 (* (/ (- _index 2) _returnvalue 2) (`KismetMathLibrary.GetPI`)))
    (`SplineComponent.SetLocationAtSplinePoint` _spline _index (`KismetMathLibrary.MakeVector` _returnvalue_x (+ (* (`KismetMathLibrary.Sin` (* _returnvalue_2 -1.0)) 500.0) 500.0) (- (* (`KismetMathLibrary.Cos` _returnvalue_2) 500.0) 600.0)) "Local" true)))

(fn `UserConstructionScript`
  (bind _returnvalue (`BaseDynamicMeshComponent.GetDynamicMesh` (`self.DynamicMeshComponent`)))
  (bind _output_get (set `self.Dynamic Mesh` _returnvalue))
  (bind _returnvalue_2 (`GeometryScriptLibrary_MeshNormalsFunctions.RecomputeNormals` _output_get (struct) false null))
  (`GeometryScriptLibrary_CollisionFunctions.SetDynamicMeshCollisionFromMesh` _returnvalue_2 (`self.DynamicMeshComponent`) (struct) null))