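; BP_NoiseControlRoom is a box-shaped zone that curses the player for making too much noise inside it.
; On overlap it binds to BP_Player's generated noise event and unbinds when the player leaves.
; Noise at or above the configured maximum level gives a configurable curse through the first player's OSPlayerState.
; The construction script sizes the box from Bounds, and a debug flag draws it and logs curse application.
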(event `self.ReceiveBeginPlay`
  (if (`self.IsDebug`)
    (`KismetSystemLibrary.DrawDebugBox` (`SceneComponent.K2_GetComponentLocation` (`self.Box`)) (`self.Bounds`) (struct) (struct) 10000.0 1.0)))

(event `self.ReceiveActorBeginOverlap`
  (params (OtherActor :type "Actor Object Reference"))
  (bind _asbp_player (cast `/Game/Player/BP_Player` OtherActor))
  (bind _output_get (set `self.Player` _asbp_player))
  (add `/Game/Player/BP_Player.GeneratedNoise` _output_get (delegate `NoiseEvaluation`)))

(event `NoiseEvaluation`
  (params (NoiseVolume :type "/Game/Weapon/LoudnessEnum Enum" :default "NewEnumerator0"))
  (if (>= (`KismetMathLibrary.Conv_ByteToInt` NoiseVolume) (`KismetMathLibrary.Conv_ByteToInt` (`self.LevelMax`)))
    (if (`self.IsDebug`)
      (`KismetSystemLibrary.PrintText` "Applying curses"))
    (bind _asosplayer_state (cast `/Game/Blueprints/OSPlayerState` (`GameplayStatics.GetPlayerState` 0)))
    (`/Game/Blueprints/OSPlayerState.GiveCurse` _asosplayer_state (`self.Curse`))))

(event `self.ReceiveActorEndOverlap`
  (params (OtherActor :type "Actor Object Reference"))
  (bind _asbp_player (cast `/Game/Player/BP_Player` OtherActor))
  (remove `/Game/Player/BP_Player.GeneratedNoise` _asbp_player (delegate `NoiseEvaluation`)))

(fn `UserConstructionScript`
  (`BoxComponent.SetBoxExtent` (`self.Box`) (`self.Bounds`) true))