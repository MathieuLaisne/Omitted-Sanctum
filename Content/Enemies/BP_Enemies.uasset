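; BP_Enemies is an enemy actor that tracks health, shows it through an HP text element and plays sounds when damaged or killed.
; It fills HP from MaxHP on BeginPlay, refreshes the text on damage, and picks a heavier hurt sound for losses of at least half MaxHP.
; IsInRange compares distance to player 0's pawn with AttackRange.
; LookAround is empty, and HPText's formatting nodes are unconnected.
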(event `self.ReceiveBeginPlay`
  (set `self.CurrentHP` (`self.MaxHP`))
  (`TextRenderComponent.K2_SetText` (`self.HP`) (`self.HPText`)))

(event `self.Die`
  (`GameplayStatics.PlaySoundAtLocation` (`self.DeathSound`) (`self.K2_GetActorLocation`) (struct) 0.5 1.0 0.0 null null null null)
  (`self.K2_DestroyActor`))

(event `self.OnDamage`
  (params (HpLost :type Integer))
  (bind _returnvalue (`self.K2_GetActorLocation`))
  (`TextRenderComponent.K2_SetText` (`self.HP`) (`self.HPText`))
  (if (>= HpLost (* (`self.MaxHP`) 0.5))
    (`GameplayStatics.PlaySoundAtLocation` (`self.GreatlyDamagedSound`) _returnvalue (struct) 0.5 1.0 0.0 null null null null)
    (else
      (`GameplayStatics.PlaySoundAtLocation` (`self.DamagedSound`) _returnvalue (struct) 0.5 1.0 0.0 null null null null))))

(event `LookAround`
  (params (Look :type Boolean)))

(fn `IsInRange`
  (returns (InRange :type Boolean))
  (bind _asosplayer_state (cast `/Game/Blueprints/OSPlayerState` (`GameplayStatics.GetPlayerState` 0))
    (:`then`
      (return (<= (`KismetMathLibrary.Vector_Distance` (`self.K2_GetActorLocation` (`PlayerState.GetPawn` _asosplayer_state)) (`self.K2_GetActorLocation`)) (`self.AttackRange`))))
    (:`CastFailed`
      (return false))))

(fn `UserConstructionScript`)