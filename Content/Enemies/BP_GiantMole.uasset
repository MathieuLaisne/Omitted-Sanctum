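; Giant mole enemy that waits for the player to overlap its Box trigger, then destroys the box and enters the Burrowed state.
; State changes drive a scalar Colour material parameter on the mesh, giving each state a value, with Idle and IntroCinematic sharing one.
; Tick writes the current surface type and state to text displays.
; The graph holds no movement or attack logic, only this trigger and state feedback.
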(event `self.Box.OnComponentBeginOverlap`
  (params (OverlappedComponent :type "PrimitiveComponent Object Reference") (OtherActor :type "Actor Object Reference") (OtherComp :type "PrimitiveComponent Object Reference") (OtherBodyIndex :type Integer) (bFromSweep :type Boolean) (SweepResult :type "HitResult Structure (by ref)"))
  (cast `/Game/Player/BP_Player` OtherActor)
  (`ActorComponent.K2_DestroyComponent` (`self.Box`))
  (`self.SetState` "Burrowed"))

(event `self.OnStateChanged`
  (params (NewState :type "EGiantMoleState Enum" :default "Idle"))
  (`MeshComponent.SetScalarParameterValueOnMaterials` (`self.Mesh`) "Colour" (select `EGiantMoleState` NewState :`Burrowed` 0.1 :`Charging` 0.3 :`SurfaceAttack` 0.5 :`Stunned` 0.7 :`Dying` 0.9 :!type "Float (single-precision)")))

(event `self.ReceiveTick`
  (params (DeltaSeconds :type "Float (single-precision)"))
  (`TextRenderComponent.K2_SetText` (`self.Surface`) (`KismetTextLibrary.Conv_StringToText` (`|GetEnumeratorNameAsString` (`self.CurrentSurfaceType`))))
  (`TextRenderComponent.K2_SetText` (`self.State`) (`KismetTextLibrary.Conv_StringToText` (`|GetEnumeratorNameAsString` (`self.CurrentState`)))))

(fn `UserConstructionScript`)