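; BP_FrozenCultist is an enemy that ties its look-around and attack behavior to the ABP_Manny animation Blueprint on its mesh.
; LookAround passes its flag to the animation Blueprint.
; Attack binds to the animation's LandedHit dispatcher and sets IsAttacking, deferring the parent class's Attack logic until that dispatcher fires.
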(event `self.LookAround`
  (params (Look :type Boolean))
  (bind _asabp_manny (cast `/Game/Characters/Mannequins/Animations/ABP_Manny` (`SkeletalMeshComponent.GetAnimInstance` (`self.Mesh`))))
  (set `/Game/Characters/Mannequins/Animations/ABP_Manny.IsLookAround` Look _asabp_manny))

(event `self.Attack`
  (bind _asabp_manny (cast `/Game/Characters/Mannequins/Animations/ABP_Manny` (`SkeletalMeshComponent.GetAnimInstance` (`self.Mesh`))))
  (add `/Game/Characters/Mannequins/Animations/ABP_Manny.LandedHit` _asabp_manny (delegate `LandedHit_Event`))
  (set `/Game/Characters/Mannequins/Animations/ABP_Manny.IsAttacking` true _asabp_manny))

(event `LandedHit_Event`
  (`parent.Attack`))

(fn `UserConstructionScript`
  (`parent.UserConstructionScript`))