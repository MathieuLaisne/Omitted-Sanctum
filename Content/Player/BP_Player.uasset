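; Player character handling Enhanced Input movement, weapons, spellcasting and HUD/pause widgets, with actor pitch derived from a gravity vector each tick.
; A screen-center box trace picks up weapons into hand slots or spellbooks onto the belt, recording their spells in the game instance.
; Spell words select a data-table element and MagicEntity class, with trace-placed previews for walls and traps.
; Running, landing and weapons emit noise, and casting triggers a speaking call.
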(event `self.ReceiveTick`
  (params (DeltaSeconds :type "Float (single-precision)"))
  (bind (_returnvalue_roll _returnvalue_pitch) (`KismetMathLibrary.BreakRotator` (`KismetMathLibrary.MakeRotFromY` (`self.Gravity`))))
  (bind (_returnvalue_roll_2 _returnvalue_pitch_2 _returnvalue_yaw) (`KismetMathLibrary.BreakRotator` (`SceneComponent.K2_GetComponentRotation` (`self.CapsuleComponent`))))
  (`self.K2_SetActorRotation` (`KismetMathLibrary.MakeRotator` _returnvalue_roll_2 _returnvalue_pitch _returnvalue_yaw)))

(event `self.ReceiveBeginPlay`
  (bind _asosplayer_controller (cast `/Game/Blueprints/OSPlayerController` (`self.GetController`)))
  (bind _returnvalue (pcsubsystem `EnhancedInputLocalPlayerSubsystem` _asosplayer_controller))
  (`/Engine/EditorBlueprintResources/StandardMacros.IsValid` _returnvalue
    (:`Is Valid`
      (`EnhancedInputSubsystemInterface.AddMappingContext` _returnvalue "/Game/OSInputMappingContext.OSInputMappingContext" 0 (struct))
      (`self.CreateMainUI`))))

(event `EnhancedInput|/Game/Blueprints/Input/IA_Attack`
  (params (ActionValue :type Boolean) (ElapsedSeconds :type "Float (double-precision)") (TriggeredSeconds :type "Float (double-precision)") (InputAction :type "InputAction Object Reference" :default "/Game/Blueprints/Input/IA_Attack.IA_Attack"))
  (bind _output (`|GetArrayItem` (`self.Weapons`) (`self.CurrentWeapon`)))
  (:`Started`
    (`/Engine/EditorBlueprintResources/StandardMacros.IsValid` _output
      (:`Is Valid`
        (`/Game/Blueprints/Weapon/BP_Weapons.Attack` _output)
        (`/Game/UI/UW_Player.AmmoChanged` (`self.UI`))))))

(event `EnhancedInput|/Game/Blueprints/Input/IA_SwitchWeapon`
  (params (ActionValue :type "Float (double-precision)") (ElapsedSeconds :type "Float (double-precision)") (TriggeredSeconds :type "Float (double-precision)") (InputAction :type "InputAction Object Reference" :default "/Game/Blueprints/Input/IA_SwitchWeapon.IA_SwitchWeapon"))
  (:`Started`
    (set `self.CurrentWeapon` (`KismetMathLibrary.Wrap` (+ (`self.CurrentWeapon`) 1) -1 1))
    (`/Game/UI/UW_Player.WeaponUpdate` (`self.UI`))
    (add `/Game/Blueprints/Weapon/BP_Weapons.NoiseGenerated` (`|GetArrayItem` (`self.Weapons`) (`self.CurrentWeapon`)) (delegate `NoiseGenerated_Event`))))

(event `NoiseGenerated_Event`
  (params (Loudness :type "/Game/Blueprints/Weapon/LoudnessEnum Enum" :default "NewEnumerator0"))
  (`self.GeneratedNoise` Loudness))

(event `EnhancedInput|/Game/Blueprints/Input/IA_GetItem`
  (params (ActionValue :type Boolean) (ElapsedSeconds :type "Float (double-precision)") (TriggeredSeconds :type "Float (double-precision)") (InputAction :type "InputAction Object Reference" :default "/Game/Blueprints/Input/IA_GetItem.IA_GetItem"))
  (bind _weapons (`self.Weapons`))
  (bind _heldspellbook (`self.HeldSpellbook`))
  (bind _currentweapon (`self.CurrentWeapon`))
  (bind _output (`|GetArrayItem` _weapons _currentweapon))
  (bind (_worldposition _worlddirection) (`GameplayStatics.DeprojectScreenToWorld` (`GameplayStatics.GetPlayerController` 0) (/ (`WidgetLayoutLibrary.GetViewportSize`) (2.0 2.0))))
  (:`Triggered`
    (bind (_outhit _returnvalue) (`KismetSystemLibrary.BoxTraceSingleByProfile` :`Start` _worldposition :`End` (+ _worldposition (* _worlddirection (1000.0 1000.0 1000.0))) :`HalfSize` (0.5 0.5 0.5) :`ProfileName` "PhysicsActor" :`DrawDebugType` "ForDuration"))
    (if _returnvalue
      (bind (_bblockinghit _binitialoverlap _time _distance _location _impactpoint _normal _impactnormal _physmat _hitactor) (`GameplayStatics.BreakHitResult` _outhit))
      (bind _asbp_weapons (cast `/Game/Blueprints/Weapon/BP_Weapons` _hitactor)
        (:`then`
          ;[1 1 1] Werapon
          (`/Engine/EditorBlueprintResources/StandardMacros.IsValid` _output
            (:`Is Valid`
              (`self.K2_DetachFromActor` _output "KeepWorld" "KeepWorld" "KeepWorld")
              (`self.SetActorEnableCollision` _output true))
            (:`Is Not Valid`
              _))
          (`KismetArrayLibrary.Array_Set` _weapons _currentweapon _asbp_weapons)
          (`self.K2_AttachToActor` _asbp_weapons self "HandL" "SnapToTarget" "SnapToTarget" "KeepRelative" false)
          (`self.SetActorEnableCollision` _asbp_weapons false)
          (add `/Game/Blueprints/Weapon/BP_Weapons.ReloadFinished` _output (delegate `UpdateUIOnReloadFinished`))
          (`/Game/UI/UW_Player.WeaponUpdate` (`self.UI`))
          (add `/Game/Blueprints/Weapon/BP_Weapons.NoiseGenerated` (`|GetArrayItem` (`self.Weapons`) (`self.CurrentWeapon`)) (delegate `NoiseGenerated_Event`)))
        (:`CastFailed`
          (bind _asbp_spellbook (cast `/Game/Blueprints/Magic/BP_Spellbook` _hitactor))
          (`/Engine/EditorBlueprintResources/StandardMacros.IsValid` _heldspellbook
            (:`Is Valid`
              ;[1 1 1] might change to inventory system
              (`self.K2_DetachFromActor` _heldspellbook "KeepWorld" "KeepWorld" "KeepWorld")
              (`self.SetActorEnableCollision` _heldspellbook true))
            (:`Is Not Valid`
              _))
          (bind _output_get (set `self.HeldSpellbook` _asbp_spellbook))
          (`self.K2_AttachToActor` _output_get self "Belt" "SnapToTarget" "SnapToTarget" "KeepRelative" true)
          (`self.SetActorEnableCollision` _output_get false)
          (bind _asosgame_instance (cast `OSGameInstance` (`GameplayStatics.GetGameInstance`)))
          (`OSGameInstance.RecordSpell` _asosgame_instance (`OSSpellbook.Spell` (`self.HeldSpellbook`)))
          (set `self.MagicDamage` (`KismetMathLibrary.Max` (`/Game/Blueprints/Magic/BP_Spellbook.Damage` _asbp_spellbook) (`self.MagicDamage`))))))))

(event `UpdateUIOnReloadFinished`
  ;[1 1 1] Werapon
  (`/Game/UI/UW_Player.AmmoChanged` (`self.UI`)))

(event `EnhancedInput|/Game/Blueprints/Input/IA_Reload`
  (params (ActionValue :type Boolean) (ElapsedSeconds :type "Float (double-precision)") (TriggeredSeconds :type "Float (double-precision)") (InputAction :type "InputAction Object Reference" :default "/Game/Blueprints/Input/IA_Reload.IA_Reload"))
  (bind _output (`|GetArrayItem` (`self.Weapons`) (`self.CurrentWeapon`)))
  (:`Started`
    (`/Engine/EditorBlueprintResources/StandardMacros.IsValid` _output
      (:`Is Valid`
        (`/Game/Blueprints/Weapon/BP_Weapons.Reload` _output)))))

(event `EnhancedInput|/Game/Blueprints/Input/IA_Movement`
  (params (ActionValue :type "Vector2D Structure") (ElapsedSeconds :type "Float (double-precision)") (TriggeredSeconds :type "Float (double-precision)") (InputAction :type "InputAction Object Reference" :default "/Game/Blueprints/Input/IA_Movement.IA_Movement"))
  (bind _returnvalue (`self.GetController`))
  (:`Triggered`
    (bind _asosplayer_state (cast `/Game/Blueprints/OSPlayerState` (`GameplayStatics.GetPlayerState` 0)))
    (bind _speedpercentage (`/Game/Blueprints/OSPlayerState.SpeedPercentage` _asosplayer_state))
    (`self.AddMovementInput` (`self.GetActorForwardVector` _returnvalue) (* _speedpercentage ActionValue_X))
    (`self.AddMovementInput` (`self.GetActorRightVector` _returnvalue) (* _speedpercentage ActionValue_Y))))

(event `EnhancedInput|/Game/Blueprints/Input/IA_LookMouse`
  (params (ActionValue :type "Vector2D Structure") (ElapsedSeconds :type "Float (double-precision)") (TriggeredSeconds :type "Float (double-precision)") (InputAction :type "InputAction Object Reference" :default "/Game/Blueprints/Input/IA_LookMouse.IA_LookMouse"))
  (:`Triggered`
    (`self.AddControllerPitchInput` ActionValue_Y)
    (`self.AddControllerYawInput` ActionValue_X)))

(event `EnhancedInput|/Game/Blueprints/Input/IA_Jump`
  (params (ActionValue :type Boolean) (ElapsedSeconds :type "Float (double-precision)") (TriggeredSeconds :type "Float (double-precision)") (InputAction :type "InputAction Object Reference" :default "/Game/Blueprints/Input/IA_Jump.IA_Jump"))
  (:`Triggered`
    (`self.Jump`)))

(event `EnhancedInput|/Game/Blueprints/Input/IA_Run`
  (params (ActionValue :type Boolean) (ElapsedSeconds :type "Float (double-precision)") (TriggeredSeconds :type "Float (double-precision)") (InputAction :type "InputAction Object Reference" :default "/Game/Blueprints/Input/IA_Run.IA_Run"))
  (:`Started`
    (set `CharacterMovementComponent.MaxWalkSpeed` 1200.0 (`self.CharacterMovement`))
    (bind _returnvalue (`GameplayStatics.SpawnSoundAtLocation` (`self.RunningSound`) (`self.K2_GetActorLocation`) (struct) 1.2 1.0 0.0 null null))
    (set `self.PlayingSound` _returnvalue)
    (`self.GeneratedNoise` "NewEnumerator2" :!label _label))
  (:`Ongoing`
    (if (== (mod ElapsedSeconds 2.0) 1.0)
      (goto _label)))
  (:`Completed`
    (`AudioComponent.Stop` (`self.PlayingSound`))
    (set `CharacterMovementComponent.MaxWalkSpeed` 600.0 (`self.CharacterMovement`))))

(event `EnhancedInput|/Game/Blueprints/Input/IA_CastSpell`
  (params (ActionValue :type Boolean) (ElapsedSeconds :type "Float (double-precision)") (TriggeredSeconds :type "Float (double-precision)") (InputAction :type "InputAction Object Reference" :default "/Game/Blueprints/Input/IA_CastSpell.IA_CastSpell"))
  (:`Triggered`
    (bind _returnvalue (`MagicHelperLibrary.SpellIsValid` (`self.Spell`)))
    (if _returnvalue
      (`self.Speaking` (`self.Spell`))
      (`self.Cast`)))
  (:`Started`
    (bind _asosgame_instance (cast `OSGameInstance` (`GameplayStatics.GetGameInstance`)))
    (bind _returnvalue_2 (`OSGameInstance.GetActiveSpellIndex` _asosgame_instance))
    (bind _outallspells (`OSGameInstance.GetAllSpells` _asosgame_instance))
    (if (`KismetArrayLibrary.Array_IsNotEmpty` _outallspells)
      (set `self.Spell` (`|GetArrayItem` _outallspells _returnvalue_2))
      (`self.SelectElement`)
      (`self.ShowPreview` true)))
  (:`Ongoing`
    (`self.MovePreview`))
  (:`Canceled`
    (`self.ShowPreview` false)))

(event `self.OnLanded`
  (params (Hit :type "HitResult Structure (by ref)"))
  (`AISense_Hearing.ReportNoiseEvent` (`self.K2_GetActorLocation`) 1.0 self 1000.0))

(event `EnhancedInput|/Game/Blueprints/Input/IA_Pause`
  (params (ActionValue :type Boolean) (ElapsedSeconds :type "Float (double-precision)") (TriggeredSeconds :type "Float (double-precision)") (InputAction :type "InputAction Object Reference" :default "/Game/Blueprints/Input/IA_Pause.IA_Pause"))
  (bind _returnvalue (`GameplayStatics.IsGamePaused`))
  (:`Completed`
    (if _returnvalue
      (`self.RemovePauseUI`)
      (`self.CreateMainUI`)
      (else
        (`self.RemoveMainUI`)
        (`self.CreatePauseUI`)))
    (`GameplayStatics.SetGamePaused` (not _returnvalue))))

(event `CreateMainUI`
  (bind _returnvalue (`|CreateWidget` "/Game/UI/UW_Player.UW_Player_C"))
  (`UserWidget.AddToViewport` _returnvalue 0)
  (set `self.UI` _returnvalue))

(event `RemoveMainUI`
  (`Widget.RemoveFromParent` (`self.UI`)))

(event `CreatePauseUI`
  (bind _returnvalue (`|CreateWidget` "/Game/UI/UW_PauseMenu.UW_PauseMenu_C"))
  (`UserWidget.AddToViewport` _returnvalue 100)
  (bind _output_get (set `self.Pause` _returnvalue))
  (`/Game/UI/UW_PauseMenu.UpdateMap` _output_get))

(event `RemovePauseUI`
  (`Widget.RemoveFromParent` (`self.Pause`)))

(event `UpdateHasPreview`
  (bind _magicpreview (`self.MagicPreview`))
  (switch `EOSMagicWord` (`.FormWord` (break `OSMagicSpell` (`self.Spell`)))
    (:`Li`
      (`StaticMeshComponent.SetStaticMesh` _magicpreview "/Engine/BasicShapes/Cube.Cube"))
    (:`Fi`
      (`StaticMeshComponent.SetStaticMesh` _magicpreview "/Engine/BasicShapes/Cylinder.Cylinder")))
  (set `self.MagicHasPreview` true))

(event `SelectElement`
  (bind _elementalword (break `OSMagicSpell` (`self.Spell`)))
  (bind _returnvalue (`|GetDataTableRow` (`self.MagicSystem`) (select `EOSMagicWord` _elementalword :`Kah` "Ice" :`Fah` "Fire" :`Tah` "Earth" :`Mah` "Electricity" :`Yah` "Plant" :!type "Name"))
    (:`then`
      (set `self.MagicEntityElement` _returnvalue)
      (set `self.MagicEntityIsSolid` (select `EOSMagicWord` _elementalword :`Kah` true :`Tah` true))
      (`self.UpdateHasPreview`))))

(event `Cast`
  (bind _currententity (`self.CurrentEntity`))
  (bind _magichaspreview (`self.MagicHasPreview`))
  (bind (_returnvalue_roll _returnvalue_pitch _returnvalue_yaw) (`KismetMathLibrary.BreakRotator` (`PlayerCameraManager.GetCameraRotation` (`GameplayStatics.GetPlayerCameraManager` 0))))
  (bind _hitlocation (`self.ForwardProjection`))
  (bind _returnvalue (`|SpawnActorFromClass` (select `EOSMagicWord` (`.FormWord` (break `OSMagicSpell` (`self.Spell`))) :`Kah` "/Script/Engine.Actor" :`Fah` "/Script/Engine.Actor" :`Tah` "/Script/Engine.Actor" :`Mah` "/Script/Engine.Actor" :`Yah` "/Script/Engine.Actor" :`Ti` "/Game/Blueprints/Magic/MagicEntities/BP_MagicWhip.BP_MagicWhip_C" :`Li` "/Game/Blueprints/Magic/MagicEntities/BP_MagicWall.BP_MagicWall_C" :`Pi` "/Game/Blueprints/Magic/MagicEntities/BP_MagicArrow.BP_MagicArrow_C" :`Bi` "/Game/Blueprints/Magic/MagicEntities/BP_MagicBall.BP_MagicBall_C" :`Fi` "/Game/Blueprints/Magic/MagicEntities/BP_MagicTrap.BP_MagicTrap_C" :`Mor` "/Script/Engine.Actor" :`Tor` "/Script/Engine.Actor" :`Kor` "/Script/Engine.Actor" :`Gor` "/Script/Engine.Actor" :`Yor` "/Script/Engine.Actor" :!type "Actor Class Reference") (`KismetMathLibrary.MakeTransform` (select `bool` _magichaspreview :`false` (+ (`self.K2_GetActorLocation`) (* (`self.GetActorForwardVector`) 100.0) (0.0 0.0 50.0) (* (`self.GetActorRightVector`) 25.0)) :`true` _hitlocation) (`KismetMathLibrary.MakeRotator` 0.0 (select `bool` _magichaspreview :`false` _returnvalue_pitch) _returnvalue_yaw)) "Undefined" "MultiplyWithRoot" self self))
  (bind _asmagic_entity (cast `MagicEntity` _returnvalue)
    (:`then`
      (bind _output_get (set `self.CurrentEntity` _asmagic_entity))
      (`MagicEntity.SetMagicElement` _output_get (`self.MagicEntityElement`))
      (`SceneComponent.SetVisibility` (`self.MagicPreview`) false false)
      (bind _asmagic_wall (cast `MagicWall` (`self.CurrentEntity`)))
      (`MagicWall.Initialize` _asmagic_wall (`self.MagicEntityIsSolid`) (`self.MagicEntityMaxHP`))
      (bind _wallmesh (`MagicWall.WallMesh` _asmagic_wall))
      (`StaticMeshComponent.SetStaticMesh` _wallmesh "/DirGravity/Assets/Cube.Cube")
      (`SceneComponent.SetWorldScale3D` _wallmesh (* (`SceneComponent.K2_GetComponentScale` (`MagicWall.EffectVolume` _asmagic_wall)) 0.9))
      (set `MagicEntity.Damage` (`self.MagicDamage`) _currententity)
      (set `MagicEntity.EffectDuration` (`KismetMathLibrary.SelectFloat` 25.0 10.0 (`KismetArrayLibrary.Array_Contains` (`.ModifierWords` (break `OSMagicSpell` (`self.Spell`))) "Tor")) _currententity))
    (:`CastFailed`
      (`self.K2_DestroyActor` _returnvalue))))

(event `MovePreview`
  (bind _magicpreview (`self.MagicPreview`))
  (bind (_returnvalue_roll _returnvalue_pitch _returnvalue_yaw) (`KismetMathLibrary.BreakRotator` (`PlayerCameraManager.GetCameraRotation` (`GameplayStatics.GetPlayerCameraManager` 0))))
  (if (`self.MagicHasPreview`)
    (bind _hitlocation (`self.ForwardProjection`))
    (`SceneComponent.K2_SetWorldLocation` _magicpreview _hitlocation false true)
    (`SceneComponent.K2_SetWorldRotation` _magicpreview (`KismetMathLibrary.MakeRotator` 0.0 0.0 _returnvalue_yaw) false false)))

(event `ShowPreview`
  (params (do :type Boolean))
  (if (`self.MagicHasPreview`)
    (`SceneComponent.SetVisibility` (`self.MagicPreview`) do false)))

(fn `ForwardProjection`
  (returns (HitLocation :type "Vector Structure"))
  (bind _camera (`self.Camera`))
  (bind _returnvalue (`SceneComponent.K2_GetComponentLocation` _camera))
  (bind _outhit (`KismetSystemLibrary.LineTraceSingleByProfile` _returnvalue (+ _returnvalue (* (`SceneComponent.GetForwardVector` _camera) 1000.0)) "BlockAll"))
  (return (`.Location` (`GameplayStatics.BreakHitResult` _outhit))))

(fn `GetCurrentWeapon`
  (returns (Weapon :type "/Game/Blueprints/Weapon/BP_Weapons Object Reference"))
  (return (`|GetArrayItem` (`self.Weapons`) (`self.CurrentWeapon`))))

(fn `GetSecondaryWeapon`
  (returns (Weapon :type "/Game/Blueprints/Weapon/BP_Weapons Object Reference"))
  (return (`|GetArrayItem` (`self.Weapons`) (`KismetMathLibrary.Wrap` (+ (`self.CurrentWeapon`) 1) -1 1))))

(fn `Gravity to World DirectionFB`
  (returns (Direction :type "Vector Structure"))
  (bind _returnvalue (`CharacterMovementComponent.GetGravityDirection` (`self.CharacterMovement`)))
  (bind (_returnvalue_roll _returnvalue_pitch _returnvalue_yaw) (`KismetMathLibrary.BreakRotator` (`GravityController.GetGravityRelativeRotation` (`self.GetControlRotation`) _returnvalue)))
  (return (`KismetMathLibrary.Conv_RotatorToVector` (`GravityController.GetGravityWorldRotation` (`KismetMathLibrary.MakeRotator` 0.0 0.0 _returnvalue_yaw) _returnvalue))))

(fn `Gravity to World DirectionRL`
  (returns (Direction :type "Vector Structure"))
  (bind _returnvalue (`CharacterMovementComponent.GetGravityDirection` (`self.CharacterMovement`)))
  (bind (_returnvalue_roll _returnvalue_pitch _returnvalue_yaw) (`KismetMathLibrary.BreakRotator` (`GravityController.GetGravityRelativeRotation` (`self.GetControlRotation`) _returnvalue)))
  (return (`KismetMathLibrary.Conv_RotatorToVector` (`GravityController.GetGravityWorldRotation` (`KismetMathLibrary.MakeRotator` _returnvalue_roll 0.0 _returnvalue_yaw) _returnvalue))))

(fn `UserConstructionScript`)