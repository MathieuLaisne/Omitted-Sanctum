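; BP_Weapons is a weapon actor, apparently a base class, that handles use and failure audio feedback and noise reporting.
; OnUsed maps the Loudness enum to a volume multiplier for GenerateNoise, which plays the use sound at the actor's location and calls NoiseGenerated with the Loudness.
; OnFailed picks a sound for no ammo, empty magazine or cooldown.
; Reload and Attack are empty events.
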(event `Reload`)

(event `Attack`)

(event `OnUsed`
  (switch `/Game/Weapon/LoudnessEnum` (`self.Loudness`)
    (:`NewEnumerator1`
      (`self.GenerateNoise` 1.0))
    (:`NewEnumerator2`
      (`self.GenerateNoise` 2.0))
    (:`NewEnumerator3`
      (`self.GenerateNoise` 5.0))))

(event `GenerateNoise`
  (params (Intensity :type "Float (double-precision)"))
  (`GameplayStatics.PlaySoundAtLocation` (`self.OnUseSound`) (`self.K2_GetActorLocation`) (struct) Intensity 1.0 0.0 null null null null)
  (`self.NoiseGenerated` (`self.Loudness`)))

(event `OnFailed`
  (params (Reason :type "/Game/Weapon/FailingReasons Enum" :default "NewEnumerator0"))
  (bind _returnvalue (`self.K2_GetActorLocation`))
  (switch `/Game/Weapon/FailingReasons` Reason
    (:`NewEnumerator0`
      (`GameplayStatics.PlaySoundAtLocation` (`self.OnNoAmmoSound`) _returnvalue (struct) 0.1 1.0 0.0 null null null null))
    (:`NewEnumerator1`
      (`GameplayStatics.PlaySoundAtLocation` (`self.OnEmptyMagSound`) (`self.K2_GetActorLocation`) (struct) 0.1 1.0 0.0 null null null null))
    (:`NewEnumerator2`
      (`GameplayStatics.PlaySoundAtLocation` (`self.OnCooldownSound`) _returnvalue (struct) 0.1 1.0 0.0 null null null null))))

(fn `UserConstructionScript`)