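; Ranged weapon Blueprint that fires a hitscan shot from its muzzle and calls Damage on any BP_Enemies hit.
; Attack checks cooldown and ammo, traces with debug drawing, then consumes ammo; Timelines serve as cooldown and reload timers.
; A non-zero AmmoMax gives a magazine that reloads by deducting a full load from player 0's OSPlayerState ammo, unchecked.
; Zero AmmoMax fires straight from that player pool.
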(event `self.ReceiveBeginPlay`
  (`parent.ReceiveBeginPlay`)
  (`TimelineComponent.SetTimelineLength` (`self.ReloadTimeline`) (`self.ReloadTime`))
  (`TimelineComponent.SetTimelineLength` (`self.CooldownTimeline`) (`self.CooldownTime`))
  (if (!= (`self.AmmoMax`) 0)
    (set `self.AmmoAmount` (`self.AmmoMax`))
    (else
      ;[1 1 1] Set To Player's Amount of Ammo
      (bind _asosplayer_state (cast `/Game/Blueprints/OSPlayerState` (`GameplayStatics.GetPlayerState` 0)))
      (set `self.AmmoAmount` (`/Game/Blueprints/OSPlayerState.Ammo` _asosplayer_state)))))

(event `self.Reload`
  (bind _ammomax (`self.AmmoMax`))
  (`Timeline|ReloadTimeline` :!via `PlayFromStart`
    (:`Finished`
      (if (!= (`self.AmmoMax`) 0)
        (set `self.AmmoAmount` _ammomax)
        ;[1 1 1] Remove Max Ammo from Player Ammo (verify if enough ammo)
        (bind _asosplayer_state (cast `/Game/Blueprints/OSPlayerState` (`GameplayStatics.GetPlayerState` 0)))
        (set `/Game/Blueprints/OSPlayerState.Ammo` (- (`/Game/Blueprints/OSPlayerState.Ammo` _asosplayer_state) _ammomax) _asosplayer_state)
        (`GameplayStatics.PlaySoundAtLocation` (`self.OnReloadSound`) (`self.K2_GetActorLocation`) (struct) 0.1 1.0 0.0 null null null null)
        (`self.ReloadFinished`)
        (else
          ;[1 1 1] Set To Player's Amount of Ammo
          (bind _asosplayer_state_2 (cast `/Game/Blueprints/OSPlayerState` (`GameplayStatics.GetPlayerState` 0)))
          (set `self.AmmoAmount` (`/Game/Blueprints/OSPlayerState.Ammo` _asosplayer_state_2)))))))

(event `self.Attack`
  (if (`self.OnCooldown`)
    _
    (elif (> (`self.AmmoAmount`) 0)
      (if (`self.OnCooldown`)
        (`self.OnFailed` "NewEnumerator2")
        (else
          (`self.OnUsed`)
          (`self.DamageLine`)
          ;[1 1 1] Ammo consume
          (if (!= (`self.AmmoMax`) 0)
            (set `self.AmmoAmount` (- (`self.AmmoAmount`) 1))
            (else
              ;;[1 1 1] Decrement Player Ammo Amount
              (bind _asosplayer_state (cast `/Game/Blueprints/OSPlayerState` (`GameplayStatics.GetPlayerState` 0)))
              (set `/Game/Blueprints/OSPlayerState.Ammo` (- (`/Game/Blueprints/OSPlayerState.Ammo` _asosplayer_state) 1) _asosplayer_state)))
          ;[1 1 1] Cooldown Time Handle
          (set `self.OnCooldown` true)
          (`Timeline|CooldownTimeline` :!via `PlayFromStart`
            (:`Finished`
              (set `self.OnCooldown` false)))))
      (elif (!= (`self.AmmoMax`) 0)
        (`self.OnFailed` "NewEnumerator1")
        (else
          (`self.OnFailed` "NewEnumerator0"))))))

(event `DamageLine`
  (bind _returnvalue (`SceneComponent.K2_GetComponentLocation` (`self.Muzzle`)))
  (bind (_outhit _returnvalue_2) (`KismetSystemLibrary.LineTraceSingleForObjects` :`Start` _returnvalue :`End` (+ _returnvalue (* (1000.0 1000.0 1000.0) (`self.GetActorForwardVector`))) :`ObjectTypes` (`self.Object Types`) :`DrawDebugType` "ForDuration"))
  (if _returnvalue_2
    (bind _asbp_enemies (cast `/Game/Enemies/BP_Enemies` (`.HitActor` (`GameplayStatics.BreakHitResult` _outhit))))
    (`/Game/Enemies/BP_Enemies.Damage` _asbp_enemies 0)))

(fn `UserConstructionScript`
  (`parent.UserConstructionScript`))